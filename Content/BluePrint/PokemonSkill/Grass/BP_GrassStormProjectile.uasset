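; Grass Storm skill projectile that spins three components (T1, T2, T3) in a ring around its Capsule.
; Tick advances the orbit angle by OrbitSpeed and places the components 120 degrees apart in XY, keeping each one's own Z.
; The orbit radius shrinks at a constant rate with no clamp, so the ring spirals inward, then expands again once the radius turns negative.
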(event EventBeginPlay)

(event Collision|EventActorBeginOverlap
  (params (OtherActor :type Actor%20Object%20Reference)))

(event EventTick
  (params (DeltaSeconds :type Float%20%28single-precision%29))
  (bind _capsule (Variables|Default|GetCapsule))
  (bind _capsule_2 (Variables|Default|GetCapsule))
  (bind _capsule_3 (Variables|Default|GetCapsule))
  (bind _returnvalue (Transformation|GetWorldLocation _capsule))
  (bind _returnvalue_2 (Transformation|GetWorldLocation _capsule_3))
  (bind _returnvalue_3 (Transformation|GetWorldLocation _capsule_2))
  (bind _output_get (Variables|Default|SetDeltaSec DeltaSeconds))
  (bind _output_get_2 (Variables|Default|SetOrbitAngle (+ (Variables|Default|GetOrbitAngle) (* _output_get (Variables|Default|GetOrbitSpeed)))))
  (bind _output_get_3 (Variables|Default|SetRadA (Math|Trig|DegreesToRadians _output_get_2)))
  (bind _output_get_4 (Variables|Default|SetRadB (+ _output_get_3 (Math|Trig|DegreesToRadians 1.2e+02))))
  (Variables|Default|SetRadC (+ _output_get_4 (Math|Trig|DegreesToRadians 1.2e+02)))
  (Transformation|SetWorldLocation (Variables|Default|GetT1) (Math|Vector|MakeVector (+ (.x _returnvalue) (* (Math|Trig|Cos(Radians) (Variables|Default|GetRadA)) (Variables|Default|GetOrbitRadius))) (+ (.y _returnvalue) (* (Math|Trig|Sin(Radians) (Variables|Default|GetRadA)) (Variables|Default|GetOrbitRadius))) (.z (Transformation|GetWorldLocation (Variables|Default|GetT1)))) false false)
  (Transformation|SetWorldLocation (Variables|Default|GetT2) (Math|Vector|MakeVector (+ (.x _returnvalue_2) (* (Math|Trig|Cos(Radians) (Variables|Default|GetRadB)) (Variables|Default|GetOrbitRadius))) (+ (.y _returnvalue_2) (* (Math|Trig|Sin(Radians) (Variables|Default|GetRadB)) (Variables|Default|GetOrbitRadius))) (.z (Transformation|GetWorldLocation (Variables|Default|GetT2)))) false false)
  (Transformation|SetWorldLocation (Variables|Default|GetT3) (Math|Vector|MakeVector (+ (.x _returnvalue_3) (* (Math|Trig|Cos(Radians) (Variables|Default|GetRadC)) (Variables|Default|GetOrbitRadius))) (+ (.y _returnvalue_3) (* (Math|Trig|Sin(Radians) (Variables|Default|GetRadC)) (Variables|Default|GetOrbitRadius))) (.z (Transformation|GetWorldLocation (Variables|Default|GetT3)))) false false)
  (Variables|Default|SetOrbitRadius (- (Variables|Default|GetOrbitRadius) (* (Variables|Default|GetDeltaSec) 1e+02))))

(fn ConstructionScript)