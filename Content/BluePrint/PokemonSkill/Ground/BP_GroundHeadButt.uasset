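; BP_GroundHeadButt is an unfinished Ground-type Pokémon skill actor, with empty BeginPlay and construction script.
; Its disconnected graph would spawn a particle emitter toward each of the actor's front, back, right and left, setting DelayTime between spawns.
; Those positions scale the whole location-plus-direction sum by Distance, not just the offset.
; The User and TargetActor checks are unwired leftovers, so none of this logic runs.
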(event EventBeginPlay)

(fn ConstructionScript)